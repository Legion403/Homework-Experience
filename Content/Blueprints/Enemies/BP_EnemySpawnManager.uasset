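; BP_EnemySpawnManager spawns enemies in waves at every BP_EnemySpawner placed in the level.
; On BeginPlay it gathers the spawners, spawns a BP_Enemy at each one's transform, gives each enemy a reference to itself and increments a live count.
; RemoveEnemyAndCheck decrements that count and, once none remain, prints a message and respawns a full wave after a short delay.
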(event Custom|Spawn%20Enemies
  (for _array_element (Variables|Default|GetSpawners)
    (bind _returnvalue (Game|SpawnActorfromClass "/Game/Blueprints/Enemies/BP_Enemy.BP_Enemy_C" (Math|Transform|MakeTransform (.location (Transformation|GetWorldTransform (Variables|/Game/Blueprints/Enemies/BP_EnemySpawner.BP_EnemySpawner_C|GetDefaultSceneRoot _array_element))) (.rotation (Transformation|GetWorldTransform (Variables|/Game/Blueprints/Enemies/BP_EnemySpawner.BP_EnemySpawner_C|GetDefaultSceneRoot _array_element))) "1.000000,1.000000,1.000000") "Undefined" "MultiplyWithRoot" 0 0)) ; Create new enemy at spawner's location and rotation
    (Variables|/Game/Blueprints/Enemies/BP_Enemy.BP_Enemy_C|SetManager _returnvalue self) ; Assign this manager to the \nmanager variable on each enemy
    (Math|Integer|IncrementInt (Variables|Default|GetCurrrentEnemyTotal))))

(event Custom|RemoveEnemyAndCheck
  (Math|Integer|DecrementInt (Variables|Default|GetCurrrentEnemyTotal)
    (:%20%20
      (if (not (> (Variables|Default|GetCurrrentEnemyTotal) 0))
        (Development|PrintString "New Enemies Spawning" true true "(R=0.062500,G=0.009857,B=0.000000,A=1.000000)" 5.0)
        (Utilities|FlowControl|Delay 5.0)
        (CallFunction|SpawnEnemies)))))

(event EventBeginPlay
  (bind _outactors (Actor|GetAllActorsOfClass "/Game/Blueprints/Enemies/BP_EnemySpawner.BP_EnemySpawner_C"))
  (Variables|Default|SetSpawners _outactors)
  (CallFunction|SpawnEnemies))

(fn ConstructionScript)