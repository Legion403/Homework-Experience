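; BP_Enemy is an enemy pawn that seeks out and damages the nearest BP_Orb_Dark.
; On BeginPlay it uses AI MoveTo toward that orb, then on arrival makes a single deduction from the orb's Health and calls its NoHealth; failure prints a debug string.
; Its own NoHealth event destroys the enemy when HealthEnemy is depleted, otherwise activates a Niagara effect.
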(event Custom|NoHealth
  (if (< (Variables|Default|GetHealthEnemy) 1)
    (Actor|DestroyActor)
    (else
      (Components|Activation|Activate (Variables|Default|GetNiagara) false))))

(event EventBeginPlay
  (bind _outactors (Actor|GetAllActorsOfClass "/Game/Env_SciFi/Blueprints/BP_Orb_Dark.BP_Orb_Dark_C"))
  (AI|AIMoveTo self "0, 0, 0" (.ReturnValue (Actor|FindNearestActor (Transformation|GetWorldLocation (Variables|Default|GetCapsule)) _outactors)) 5.0 false
    (:OnSuccess
      (bind _asbp_orb_dark (Utilities|Casting|CastToBP_Orb_Dark (.ReturnValue (Actor|FindNearestActor (Transformation|GetWorldLocation (Variables|Default|GetCapsule)) _outactors))))
      (Variables|/Game/Env_SciFi/Blueprints/BP_Orb_Dark.BP_Orb_Dark_C|SetHealth _asbp_orb_dark (- (Variables|/Game/Env_SciFi/Blueprints/BP_Orb_Dark.BP_Orb_Dark_C|GetHealth _asbp_orb_dark) 10))
      (Default|NoHealth _asbp_orb_dark))
    (:OnFail
      (Development|PrintString "Hello"))))

(event Collision|EventActorBeginOverlap
  (params (OtherActor :type Actor%20Object%20Reference)))

(event EventTick
  (params (DeltaSeconds :type Float%20%28single-precision%29)))

(fn ConstructionScript)