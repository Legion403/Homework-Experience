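; Enemy spawner actor that places BP_ENEMyAIFR enemies into the level.
; On BeginPlay it waits briefly, then spawns three enemies in a fixed timed sequence of chained Delay nodes, with no loop or trigger.
; Each spawn uses the Box component's world transform and always spawns regardless of collision.
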(event EventBeginPlay
  (Utilities|FlowControl|Delay 0.2)
  (Game|SpawnActorfromClass "/Game/LegionsLevel/BluePrints/Enemy/BP_ENEMyAIFR.BP_ENEMyAIFR_C" (Transformation|GetWorldTransform (Variables|Default|GetBox)) "AlwaysSpawn" "MultiplyWithRoot" 0 0)
  (Utilities|FlowControl|Delay 1e+01)
  (Game|SpawnActorfromClass "/Game/LegionsLevel/BluePrints/Enemy/BP_ENEMyAIFR.BP_ENEMyAIFR_C" (Transformation|GetWorldTransform (Variables|Default|GetBox)) "AlwaysSpawn" "MultiplyWithRoot" 0 0)
  (Utilities|FlowControl|Delay 1e+01)
  (Game|SpawnActorfromClass "/Game/LegionsLevel/BluePrints/Enemy/BP_ENEMyAIFR.BP_ENEMyAIFR_C" (Transformation|GetWorldTransform (Variables|Default|GetBox)) "AlwaysSpawn" "MultiplyWithRoot" 0 0))

(event Collision|EventActorBeginOverlap
  (params (OtherActor :type Actor%20Object%20Reference)))

(event EventTick
  (params (DeltaSeconds :type Float%20%28single-precision%29)))

(fn ConstructionScript)